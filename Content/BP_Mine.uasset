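; BP_Mine is a proximity mine that explodes when an actor implementing HealthInterface, other than a TopDownCharacter, overlaps its Box.
; It plays a 2D explosion sound and calls TopDownGameState's SpawnAOE for a line-of-sight radial hit, credited to the player character.
; A delegate event sends a fixed DamageMessage to each hit actor.
; The mine does not destroy or disable itself here.
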(event `self.Box.OnComponentBeginOverlap`
  (params (OverlappedComponent :type "PrimitiveComponent Object Reference") (OtherActor :type "Actor Object Reference") (OtherComp :type "PrimitiveComponent Object Reference") (OtherBodyIndex :type Integer) (bFromSweep :type Boolean) (SweepResult :type "HitResult Structure (by ref)"))
  (if (`KismetSystemLibrary.DoesImplementInterface` OtherActor "/Game/HealthInterface.HealthInterface_C")
    (cast `/Game/TopDownBP/Blueprints/TopDownCharacter` OtherActor
      (:`CastFailed`
        (bind _astop_down_game_state (cast `/Game/TopDownGameState` (`GameplayStatics.GetGameState`)))
        (`GameplayStatics.PlaySound2D` "/Game/Music/MineExplosion.MineExplosion" 1.0 1.0 0.0 null null)
        (`/Game/TopDownGameState.SpawnAOE` _astop_down_game_state (`self.K2_GetActorLocation`) 400.0 true (`GameplayStatics.GetPlayerCharacter` 0) (delegate `CustomEvent_0`) 2.5 (struct :`R` 1.0 :`G` 0.818636 :`A` 1.0))))))

(event `CustomEvent_0`
  (params (`Hit Actor` :type "Actor Object Reference"))
  (message `/Game/HealthInterface.Damage` `Hit Actor` 100.0))

(fn `UserConstructionScript`)