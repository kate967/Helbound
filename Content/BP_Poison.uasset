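; BP_Poison is a poison ability actor that applies a one-shot area effect around its spawn location.
; On BeginPlay it has the TopDownGameState spawn an AOE credited to player 0, with a debug draw and a hit callback, then plays the Poison flipbook.
; The callback sends each hit actor a damage message that currently evaluates to zero.
; The actor destroys itself just before the flipbook ends.
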(event `self.ReceiveBeginPlay`
  ;[1 1 1] AOE Heal
  (bind _astop_down_game_state (cast `/Game/TopDownGameState` (`GameplayStatics.GetGameState`)))
  (`/Game/TopDownGameState.SpawnAOE` _astop_down_game_state (`self.K2_GetActorLocation`) 400.0 false (`GameplayStatics.GetPlayerCharacter` 0) (delegate `CustomEvent`) 0.1 (struct :`R` 0.330041 :`G` 0.096291 :`B` 0.494792 :`A` 1.0))
  (`PaperFlipbookComponent.SetFlipbook` (`self.AbilityFlipbook`) "/Game/Flipbooks/Abilities/Poison.Poison")
  (`KismetSystemLibrary.Delay` (- (`PaperFlipbookComponent.GetFlipbookLength` (`self.AbilityFlipbook`)) 0.1))
  (`self.K2_DestroyActor`))

(event `CustomEvent`
  (params (`Hit Actor` :type "Actor Object Reference"))
  ;[1 1 1] AOE Heal
  (message `/Game/HealthInterface.Damage` `Hit Actor` (* 0.0 50.0)))

(fn `UserConstructionScript`)